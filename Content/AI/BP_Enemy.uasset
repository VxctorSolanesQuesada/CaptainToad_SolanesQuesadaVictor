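; BP_Enemy is an enemy actor that deals contact damage and drops a coin when killed.
; Capsule hits remove health from any actor with a BP_HealthComponent, throttled by a two-second cooldown flag.
; Its own health component's OnDeath event triggers EnemyDie, which enables capsule physics, launches the body away from the killer, then destroys it shortly after and spawns a BP_Coin at its location.
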(event `EnemyDie`
  (params (Killer :type "Actor Object Reference"))
  (bind _capsulecomponent (`self.CapsuleComponent`))
  (`PrimitiveComponent.SetSimulatePhysics` _capsulecomponent true)
  (`PrimitiveComponent.AddImpulse` _capsulecomponent (* (`KismetMathLibrary.Normal` (- (`self.K2_GetActorLocation`) (`self.K2_GetActorLocation` Killer))) 30000.0) "None" false)
  (`KismetSystemLibrary.Delay` 0.5)
  (`self.K2_DestroyActor`)
  (`|SpawnActorFromClass` "/Game/Blueprints/BP_Coin.BP_Coin_C" (`KismetMathLibrary.Conv_VectorToTransform` (`self.K2_GetActorLocation`)) "Undefined" "MultiplyWithRoot" null null))

(event `self.ReceiveBeginPlay`
  (add `/Game/Blueprints/BP_HealthComponent.OnDeath` (`self.BP_HealthComponent`) (delegate `EnemyDie`)))

(event `self.CapsuleComponent.OnComponentHit`
  (params (HitComponent :type "PrimitiveComponent Object Reference") (OtherActor :type "Actor Object Reference") (OtherComp :type "PrimitiveComponent Object Reference") (NormalImpulse :type "Vector Structure") (Hit :type "HitResult Structure (by ref)"))
  (bind _returnvalue (`self.GetComponentByClass` OtherActor "/Game/Blueprints/BP_HealthComponent.BP_HealthComponent_C"))
  (if (`self.DamageTimer`)
    _
    (elif (`KismetSystemLibrary.IsValid` _returnvalue)
      (`/Game/Blueprints/BP_HealthComponent.RemoveHealth` _returnvalue 1.0 null)
      (set `self.DamageTimer` true)
      (`KismetSystemLibrary.Delay` 2.0)
      (set `self.DamageTimer` false))))

(fn `UserConstructionScript`)