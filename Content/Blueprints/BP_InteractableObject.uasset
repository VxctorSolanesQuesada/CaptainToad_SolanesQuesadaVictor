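; BP_InteractableObject is an interactable object that sends on/off signals to a set of target objects.
; SwitchOn and SwitchOff loop over TargetObjects and send SwitchStateMessage with true or false to each one implementing the I_SignarReciever interface, so receivers need no casts.
; The event graph is empty, and nothing in this Blueprint calls either function.
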(fn `SwitchOff`
  (for _array_element (`self.TargetObjects`)
    (if (`KismetSystemLibrary.DoesImplementInterface` _array_element "/Game/Blueprints/I_SignarReciever.I_SignarReciever_C")
      (message `/Game/Blueprints/I_SignarReciever.SwitchState` _array_element false))))

(fn `SwitchOn`
  (for _array_element (`self.TargetObjects`)
    (if (`KismetSystemLibrary.DoesImplementInterface` _array_element "/Game/Blueprints/I_SignarReciever.I_SignarReciever_C")
      (message `/Game/Blueprints/I_SignarReciever.SwitchState` _array_element true))))