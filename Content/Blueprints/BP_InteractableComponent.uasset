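; BP_InteractableComponent is a physics barrel that the player character can pick up and throw.
; PickupObject turns off the barrel's physics and attaches it to the PickupPlace on BP_ThirdPersonCharacter.
; ThrowObject restores physics, detaches it and applies a strong impulse along the character capsule's forward vector.
; Both functions find the character by casting player pawn 0; nothing in this Blueprint calls them.
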(event `CustomEvent`)

(fn `PickupObject`
  (bind _asbp_third_person_character (cast `/Game/Blueprints/BP_ThirdPersonCharacter` (`GameplayStatics.GetPlayerPawn` 0))
    (:`then`
      (`PrimitiveComponent.SetSimulatePhysics` (`self.barrel`) false)
      (`self.K2_AttachToComponent` (`/Game/Blueprints/BP_ThirdPersonCharacter.PickupPlace` _asbp_third_person_character) "None" "SnapToTarget" "SnapToTarget" "KeepRelative"))
    (:`CastFailed`
      (`KismetSystemLibrary.PrintString` "falla cast PJ en objeto inte"))))

(fn `ThrowObject`
  (bind _barrel (`self.barrel`))
  (bind _asbp_third_person_character (cast `/Game/Blueprints/BP_ThirdPersonCharacter` (`GameplayStatics.GetPlayerPawn` 0)))
  (`PrimitiveComponent.SetSimulatePhysics` _barrel true)
  (`self.K2_DetachFromActor` "KeepRelative")
  (`PrimitiveComponent.AddImpulse` _barrel (* (`SceneComponent.GetForwardVector` (`Character.CapsuleComponent` _asbp_third_person_character)) 10000.0) "None" false))

(fn `UserConstructionScript`)