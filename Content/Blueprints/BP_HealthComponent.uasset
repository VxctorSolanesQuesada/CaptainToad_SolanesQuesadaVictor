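; Health component that tracks an owner's health and broadcasts changes through event dispatchers.
; AddHealth raises Health up to MaxHealth, firing OnCurar only when the heal does not exceed the cap, always with AmountAdded at zero.
; RemoveHealth subtracts damage without clamping, fires OnHit, then fires OnDeath with the damage dealer whenever Health is zero or below.
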(fn `AddHealth`
  (params (Amount :type "Float (double-precision)"))
  (bind _returnvalue (+ Amount (`self.Health`)))
  (if (<= _returnvalue (`self.MaxHealth`))
    (bind _output_get (set `self.Health` _returnvalue))
    (`self.OnCurar` _output_get)
    (else
      (set `self.Health` (`self.MaxHealth`)))))

(fn `RemoveHealth`
  (params (Amount :type "Float (double-precision)") (DmgDealer :type "Actor Object Reference"))
  (bind _output_get (set `self.Health` (- (`self.Health`) Amount)))
  (`self.OnHit` _output_get Amount)
  (if (<= _output_get 0.0)
    (`self.OnDeath` DmgDealer)))